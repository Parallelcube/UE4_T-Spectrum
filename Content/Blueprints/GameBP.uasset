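; GameBP is an actor that bootstraps the game's audio and player UI when play begins.
; It constructs an AudioManagerBP object with itself as outer, stores it and initializes it.
; It then creates the UI_Player widget, passes it a reference to itself and tells it to show.
; The construction script and overlap event are empty.
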(event `self.ReceiveBeginPlay`
  ;[0.004176 0.006887 0.02604] Initialization
  (`self.InitializeAudioManager`)
  (`self.InitializeUI`)
  (`/Game/Blueprints/UI_Player.ShowUI` (`self.UI_Player`)))

(fn `InitializeAudioManager`
  ;[0 0.02604 0.01004] Initialize Audio manager
  (bind _returnvalue (`|GenericCreateObject` "/Game/Blueprints/AudioManagerBP.AudioManagerBP_C" self))
  (bind _output_get (set `self.AudioManagerBP` _returnvalue))
  (`AudioManager.InitializeManager` _output_get))

(fn `InitializeUI`
  (bind _returnvalue (`|CreateWidget` "/Game/Blueprints/UI_Player.UI_Player_C"))
  (bind _output_get (set `self.UI_Player` _returnvalue))
  (`/Game/Blueprints/UI_Player.SetGameBP` _output_get self))

(fn `UserConstructionScript`)